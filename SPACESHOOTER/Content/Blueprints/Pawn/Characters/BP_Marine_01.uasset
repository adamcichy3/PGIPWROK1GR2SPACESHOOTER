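; BP_Marine_01 is a player marine character that moves along world axes, aims by mouse movement and creates its HUD widget on BeginPlay.
; Each tick, mouse velocity above a dead-zone threshold sets a yaw that the control rotation interpolates toward, so aim follows swipe direction rather than cursor position.
; Fire input toggles the rifle muzzle-flash effect and firing sounds; it handles no projectiles or damage.
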(event EventTick
  (params (DeltaSeconds :type Float%20%28single-precision%29))
  (CallFunction|UpdateRotation))

(event EventBeginPlay
  (bind _returnvalue (UserInterface|CreateWidget "/Game/UMG/WB_HUD_01.WB_HUD_01_C" 0 self))
  (UserInterface|Viewport|AddtoViewport _returnvalue 0))

(event Input|ActionEvents|InputActionFire
  (params (Key :type Key%20Structure :default "None"))
  (:Pressed
    (CallFunction|StartFire))
  (:Released
    (CallFunction|StopFire 0.0)))

(event Input|AxisEvents|InputAxisMoveForwardBack
  (params (AxisValue :type Float%20%28single-precision%29))
  (Pawn|Input|AddMovementInput "1.000000, 0, 0" AxisValue false))

(event Input|AxisEvents|InputAxisMoveLeftRight
  (params (AxisValue :type Float%20%28single-precision%29))
  (Pawn|Input|AddMovementInput "0,1.000000, 0" AxisValue false))

(fn ConstructionScript)

(fn UpdateRotation
  (bind _returnvalue (Game|GetPlayerController 0))
  (bind _returnvalue_2 (CallFunction|MouseVelocity))
  (bind (_x _y) (Math|Vector2D|BreakVector2D _returnvalue_2))
  (if (CallFunction|IsDeadZone)
    (Pawn|SetControlRotation _returnvalue (Math|Interpolation|RInterpTo (Pawn|GetControlRotation _returnvalue :!class /Script/Engine.Controller) (Math|Rotator|MakeRotator 0.0 0.0 (Class|KismetMathLibrary|DegAtan2 _x _y)) (Utilities|Time|GetWorldDeltaSeconds) (Variables|Default|GetInterp%20Speed)))))

(fn MouseVelocity
  (bind _returnvalue (Game|GetPlayerController 0))
  (bind (_deltax _deltay) (Class|PlayerController|GetInputMouseDelta _returnvalue))
  (return (/ (Math|Vector2D|MakeVector2D _deltax _deltay) (Utilities|Time|GetWorldDeltaSeconds))))

(fn IsDeadZone
  (return (> (Math|Vector2D|Vector2DLength (CallFunction|MouseVelocity)) (LocalVariables|GetDeadZone))))

(fn StartFire
  (bind _p_assaultrifle_mf (Variables|Default|GetP_AssaultRifle_MF))
  (Components|Activation|Activate _p_assaultrifle_mf false)
  (bind _returnvalue (Audio|SpawnSound2D "/Game/Sounds/Weapon_AssaultRifle/Stereo/SC_Fire_01.SC_Fire_01" 1.0 1.0 0.0 0))
  (Variables|Default|SetAudio_Fire_01 _returnvalue)
  (return _p_assaultrifle_mf))

(fn StopFire
  (params (self2 :type Float%20%28single-precision%29))
  (Components|Activation|Deactivate (Variables|Default|GetP_AssaultRifle_MF))
  (Audio|Components|Audio|Stop (Variables|Default|GetAudio_Fire_01))
  (Audio|SpawnSound2D "/Game/Sounds/Weapon_AssaultRifle/Stereo/SC_EndFire_01.SC_EndFire_01" 1.0 1.0 0.0 0))